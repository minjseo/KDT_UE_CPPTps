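; BP_Only_Enemy is an enemy actor with health, an HP bar widget and an FSM that handles its states.
; Each tick it sets the HP bar's world rotation to a value supplied by the FSM.
; DamageProcess subtracts damage from current HP, updates the bar's percent, then switches the FSM to one of two states depending on whether any HP remains.
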(event EventBeginPlay
  (Variables|Default|SetFSM (Variables|Default|GetFSM))
  (Variables|Default|SetcurrHP (Variables|Default|GetmaxHP)))

(event Collision|EventActorBeginOverlap
  (params (OtherActor :type Actor%20Object%20Reference)))

(event EventTick
  (params (DeltaSeconds :type Float%20%28single-precision%29))
  (bind _rot (Default|GetRotHPBar (Variables|Default|GetFSM)))
  (Transformation|SetWorldRotation (Variables|Default|GetHPBar) _rot false false))

(fn ConstructionScript)

(fn DamageProcess
  (params (damage :type Integer))
  (Variables|Default|SetcurrHP (- (Variables|Default|GetcurrHP) damage))
  ;[1 1 1] HPBar Widget 갱신
  (bind _asbp_enemy_hpbar (Utilities|Casting|CastToBP_EnemyHPBar (UserInterface|GetWidget (Variables|Default|GetHPBar))))
  (Progress|SetPercent (Variables|/Script/CPPTps.EnemyHPBar|GetHPBar _asbp_enemy_hpbar) (/ (Math|Float|MakeLiteralFloat (Math|Conversions|ToFloat(Integer) (Variables|Default|GetcurrHP))) (Variables|Default|GetmaxHP)))
  (if (> (Variables|Default|GetcurrHP) 0)
    (Default|ChangeState (Variables|Default|GetFSM) "NewEnumerator3")
    (else
      (Default|ChangeState (Variables|Default|GetFSM) "NewEnumerator4"))))