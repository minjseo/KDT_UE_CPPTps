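; Enemy AI state machine component for BP_Only_Enemy that patrols around its spawn, chases and attacks the player, and returns when beyond its move range.
; Tick dispatches per-state updates, moving through AIController navigation and detecting the player by distance, cosine view-angle and line-of-sight trace.
; ChangeState stops movement, syncs the AnimBP, randomizes attacks, damage montages and patrol points, and handles death.
; GetRotHPBar supplies a camera-facing health bar rotation.
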(event EventBeginPlay
  ;[1 1 1] 플레이어 찾자
  (bind _returnvalue (Actor|GetActorOfClass "/Game/Blueprints/OnlyBlueprints/BP_Only_TpsPlayer.BP_Only_TpsPlayer_C"))
  (Variables|Default|Settarget _returnvalue)
  ;[1 1 1] 나의 액터를 찾자
  (bind _asbp_only_enemy (Utilities|Casting|CastToBP_Only_Enemy (Components|GetOwner)))
  (Variables|Default|SetmyActor _asbp_only_enemy)
  ;[1 1 1] 나의 Animation Blueprint 가져오자
  (bind _asabp_only_enemy (Utilities|Casting|CastToABP_Only_Enemy (Components|SkeletalMesh|GetAnimInstance (Variables|/Script/Engine.Character|GetMesh (Variables|Default|GetmyActor)))))
  (Variables|Default|Setanim _asabp_only_enemy)
  ;[1 1 1] AIController 를 가져오자
  (bind _asaicontroller (Utilities|Casting|CastToAIController (Pawn|GetController (Variables|Default|GetmyActor))))
  (Variables|Default|Setai _asaicontroller)
  ;[1 1 1] 시야각을 cos(시야각) 으로 하자
  (Variables|Default|SetviewAngle (Math|Trig|Cos(Degrees) (* (Variables|Default|GetviewAngle) 0.5)))
  ;[1 1 1] 처음 위치 저장
  (Variables|Default|SetoriginPos (Transformation|GetActorLocation (Variables|Default|GetmyActor))))

(event EventTick
  (params (DeltaSeconds :type Float%20%28single-precision%29))
  (Utilities|IsValid (Variables|Default|Gettarget)
    (:Is%20Valid
      (switch Utilities|FlowControl|Switch|SwitchonBP_Only_EnemyState (Variables|Default|GetcurrState)
        (:NewEnumerator0
          (CallFunction|UpdateIdle))
        (:NewEnumerator1
          (CallFunction|UpdateMove))
        (:NewEnumerator2
          (CallFunction|UpdateAttack))
        (:NewEnumerator3
          (CallFunction|UpdateDamage))
        (:NewEnumerator5
          (CallFunction|UpdateAttackDelay))
        (:NewEnumerator6
          (CallFunction|UpdateReturn))
        (:NewEnumerator7
          (CallFunction|UpdatePatrol))))))

(fn UpdateIdle
  (bind _can (CallFunction|CanTrace))
  (if _can
    (CallFunction|ChangeState "NewEnumerator1")
    (else
      (bind _complete (CallFunction|IsWaitComplete 2.0))
      (if _complete
        (CallFunction|ChangeState "NewEnumerator7")))))

(fn UpdateMove
  ;[1 1 1] 만약에 움직일 수 있는 범위를 넘어갔다면 상태를 RETURN 으로 하자
  (if (> (Math|Vector|Distance(Vector) (Variables|Default|GetoriginPos) (Transformation|GetActorLocation (Variables|Default|GetmyActor))) (Variables|Default|GetmoveRange))
    (CallFunction|ChangeState "NewEnumerator6")
    (else
      ;[1 1 1] 플레이어를 향하는 방향을 구하자  , 플레이어와의 거리도 구하자
      (bind _output_get (LocalVariables|Setdir (- (Transformation|GetActorLocation (Variables|Default|Gettarget)) (Transformation|GetActorLocation (Variables|Default|GetmyActor)))))
      (LocalVariables|Setdist (Math|Vector|VectorLength _output_get))
      ;[1 1 1] Navigation 기능으로 목적지까지 가라
      (AI|Navigation|MovetoLocation (Variables|Default|Getai) (Transformation|GetActorLocation (Variables|Default|Gettarget)) -1.0 true true false true 0)
      ;[1 1 1] 만약에 플레이어가 AttactRange 에 들어왔다면 ATTACK 상태로 바꿔라
      (if (< (LocalVariables|Getdist) (Variables|Default|GetatttackRange))
        (CallFunction|ChangeState "NewEnumerator2")))))

(fn UpdateAttackDelay
  ;[1 1 1] 시간을 흐르게 하자
  (bind _output_get (Variables|Default|SetcurrTime (+ (Variables|Default|GetcurrTime) (Utilities|Time|GetWorldDeltaSeconds))))
  (if (> _output_get (Variables|Default|GetattackDelayTime))
    (Variables|Default|SetcurrTime 0.0)
    ;[1 1 1] 만약에 Attack Range 플레어가 있다면 공격해라!!
    (if (< (Math|Vector|Distance(Vector) (Transformation|GetActorLocation (Variables|Default|Gettarget)) (Transformation|GetActorLocation (Variables|Default|GetmyActor))) (Variables|Default|GetatttackRange))
      (CallFunction|ChangeState "NewEnumerator2")
      (else
        ;[1 1 1] 그렇지않고 만약에 TraceRange 에 있다고 시야각에 들어와 있다면 쫓아가라 (상태를 MOVE)
        (bind _can (CallFunction|CanTrace))
        (if _can
          (CallFunction|ChangeState "NewEnumerator1")
          (else
            ;[1 1 1] 그렇지 않으면 IDLE 상태로 가라
            (CallFunction|ChangeState "NewEnumerator0")))))))

(fn ChangeState
  (params (state :type BP_Only_EnemyState%20Enum :default "NewEnumerator0"))
  (bind _myactor (Variables|Default|GetmyActor))
  (Development|PrintString (Utilities|String|Append (Utilities|String|EnumtoString (Variables|Default|GetcurrState)) "---------->" (Utilities|String|EnumtoString state)))
  (AI|Navigation|StopMovement (Variables|Default|Getai)) ; 네이게이션 동작 멈춰!
  (bind _output_get (Variables|Default|SetcurrState state)) ; 현재 상태 갱신
  (bind _output_get_2 (Variables|/Game/Blueprints/OnlyBlueprints/ABP_Only_Enemy.ABP_Only_Enemy_C|Setstate (Variables|Default|Getanim) _output_get)) ; 애니메이션 상태 갱신
  (Variables|Default|SetcurrTime 0.0)
  (switch Utilities|FlowControl|Switch|SwitchonBP_Only_EnemyState _output_get_2
    (:NewEnumerator2
      ;[1 1 1] 랜덤한 공격 모션을 선택하자
      (Variables|/Game/Blueprints/OnlyBlueprints/ABP_Only_Enemy.ABP_Only_Enemy_C|SetattackType (Variables|Default|Getanim) (Utilities|Enum|ByteToEnumBP_Only_AttackType (Math|Conversions|ToByte(Integer) (Math|Random|RandomIntegerinRange 0 1)))))
    (:NewEnumerator3
      ;[1 1 1] 랜덤한 피격 모션 (Montage 이용)
      (Animation|PlayAnimMontage (Variables|Default|GetmyActor) "/Game/Blueprints/OnlyBlueprints/EnemyMontage.EnemyMontage" 1.0 (Utilities|String|StringToName (Utilities|String|Append (Utilities|String|MakeLiteralString "Damage0") (Utilities|String|ToString(Integer) (Math|Random|RandomIntegerinRange 1 2))))))
    (:NewEnumerator4
      ;[1 1 1] 죽음 상태 설정
      (Animation|PlayAnimMontage _myactor "/Game/Blueprints/OnlyBlueprints/EnemyMontage.EnemyMontage" 1.0 "Die")
      (Collision|SetCollisionEnabled (Variables|/Script/Engine.Character|GetCapsuleComponent _myactor) "NoCollision"))
    (:NewEnumerator7
      ;[1 1 1] 처음 위치 기준으로 반경 500 cm 안의 랜덤 위치를 계산하고 그 위치로 이동해라
      (bind _output_get_3 (Variables|Default|SetpatrlPos (+ (* (Math|Vector|GetForwardVector (Math|Rotator|MakeRotator 0.0 0.0 (Math|Conversions|ToFloat(Integer) (Math|Random|RandomIntegerinRange 0 359)))) (Math|Random|RandomFloatinRange 1e+02 5e+02)) (Variables|Default|GetoriginPos))))
      (AI|Navigation|MovetoLocation (Variables|Default|Getai) _output_get_3 -1.0 true true false true 0))))

(fn UpdateDamage
  (bind _output_get (Variables|Default|SetcurrTime (+ (Variables|Default|GetcurrTime) (Utilities|Time|GetWorldDeltaSeconds))))
  (if (> _output_get (Variables|Default|GetdamageDelayTime))
    (CallFunction|ChangeState "NewEnumerator0")))

(fn UpdateAttack
  (CallFunction|ChangeState "NewEnumerator5"))

(fn CanTrace
  ;[1 1 1] 플레이어와의 거리 체크
  (bind _output_get (LocalVariables|Setdir (- (Transformation|GetActorLocation (Variables|Default|Gettarget)) (Transformation|GetActorLocation (Variables|Default|GetmyActor)))))
  (if (< (Math|Vector|VectorLength _output_get) (Variables|Default|GettraceRange))
    ;[1 1 1] 시야각 체크
    (if (> (Math|Vector|DotProduct (Math|Vector|Normalize (LocalVariables|Getdir)) (Transformation|GetActorForwardVector (Variables|Default|GetmyActor))) (Variables|Default|GetviewAngle))
      ;[1 1 1] 중간에 장애물이 존재 하니?
      (bind (_outhit _returnvalue) (Collision|LineTraceByChannel (Transformation|GetActorLocation (Variables|Default|GetmyActor)) (Transformation|GetActorLocation (Variables|Default|Gettarget)) "TraceTypeQuery1" false 0 "None"))
      (if _returnvalue
        (return (Utilities|String|Contains (Utilities|GetDisplayName (.hitactor _outhit)) "Player")))
      (else
        (return false)))
    (else
      (return false))))

(fn UpdateReturn
  (bind _returnvalue (AI|Navigation|MovetoLocation (Variables|Default|Getai) (Variables|Default|GetoriginPos) -1.0 true true false true 0))
  (if (Utilities|Enum|Equal(Enum) _returnvalue "AlreadyAtGoal")
    (CallFunction|ChangeState "NewEnumerator0")))

(fn UpdatePatrol
  (if (< (Math|Vector|Distance(Vector) (Transformation|GetActorLocation (Variables|Default|GetmyActor)) (Variables|Default|GetpatrlPos)) 5e+01)
    (CallFunction|ChangeState "NewEnumerator0")))

(fn IsWaitComplete
  (params (delay :type Float%20%28double-precision%29))
  (bind _output_get (Variables|Default|SetcurrTime (+ (Variables|Default|GetcurrTime) (Utilities|Time|GetWorldDeltaSeconds))))
  (return (> _output_get delay)))

(fn GetRotHPBar
  (return (Math|Rotator|MakeRotfromXZ (* (Math|Vector|GetForwardVector (Variables|/Game/Blueprints/OnlyBlueprints/BP_Only_TpsPlayer.BP_Only_TpsPlayer_C|GetCamera (Variables|Default|Gettarget))) (Math|Float|MakeLiteralFloat -1.0)) (Math|Vector|GetUpVector (Variables|/Game/Blueprints/OnlyBlueprints/BP_Only_TpsPlayer.BP_Only_TpsPlayer_C|GetCamera (Variables|Default|Gettarget))))))